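; BP_Bullet_Main is a gun projectile actor that kills a third-person character on impact.
; On BeginPlay it sets local velocity on its ProjectileMovement from BulletSpeed, adding random spread on the Z axis only, scaled by RandomlyBulletVector.
; When its static mesh hits something, it destroys itself, prints the hit actor's name and calls PhysicsDead if that actor is a BP_ThirdPersonCharacter.
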(event OnComponentHit(StaticMesh)
  (params (HitComponent :type Primitive%20Component%20Object%20Reference) (OtherActor :type Actor%20Object%20Reference) (OtherComp :type Primitive%20Component%20Object%20Reference) (NormalImpulse :type Vector :default "0, 0, 0") (Hit :type Hit%20Result%20Structure%20%28by%20ref%29))
  (Actor|DestroyActor)
  (Development|PrintString (Utilities|GetDisplayName OtherActor))
  (bind _asbp_third_person_character (Utilities|Casting|CastToBP_ThirdPersonCharacter OtherActor))
  (Default|PhysicsDead _asbp_third_person_character))

(event EventBeginPlay
  (bind _bulletspeed (Variables|Default|GetBulletSpeed))
  (bind _randomlybulletvector (Variables|Default|GetRandomlyBulletVector))
  (bind _returnvalue (/ _randomlybulletvector 2.0))
  ;[1 1 1] RandomlyBulletVector
  (Game|Components|ProjectileMovement|SetVelocityinLocalSpace (Variables|Default|GetProjectileMovement) (Math|Vector|MakeVector _bulletspeed 0.0 (* _bulletspeed (Math|Random|RandomFloatinRange (- _returnvalue _randomlybulletvector) _returnvalue)))))

(event Collision|EventActorBeginOverlap
  (params (OtherActor :type Actor%20Object%20Reference)))

(event EventTick
  (params (DeltaSeconds :type Float%20%28single-precision%29)))

(fn ConstructionScript)