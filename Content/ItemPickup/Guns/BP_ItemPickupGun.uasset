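; Gun item pickup Blueprint that handles firing by spawning projectiles.
; The Fire event stores the passed player rotation, then loops over the pellet count to spawn the configured bullet class just ahead of the pickup object along that facing.
; All pellets share the same position and rotation with no spread in this graph, relying on collision handling that adjusts placement but always spawns.
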(event Custom|Fire
  (params (PlayerRotation :type Rotator))
  (Variables|Default|SetPlayerRotation PlayerRotation)
  (for _index (range 0 (Variables|Default|GetPelletsNum))
    (Game|SpawnActorfromClass (Variables|Default|GetBulletClass) (Math|Transform|MakeTransform (+ (Transformation|GetWorldLocation (Variables|Default|GetPickupObj)) (* (Math|Vector|GetForwardVector (Variables|Default|GetPlayerRotation)) 5e+01)) (Variables|Default|GetPlayerRotation) "1.000000,1.000000,1.000000") "AdjustIfPossibleButAlwaysSpawn" "MultiplyWithRoot" 0 0)))

(event EventBeginPlay
  (|CallParentFunction) ; This node is disabled and will not be called.\nDrag off pins to build functionality.
)

(event Collision|EventActorBeginOverlap
  (params (OtherActor :type Actor%20Object%20Reference))
  (|CallParentFunction OtherActor) ; This node is disabled and will not be called.\nDrag off pins to build functionality.
)

(event EventTick
  (params (DeltaSeconds :type Float%20%28single-precision%29))
  (|CallParentFunction DeltaSeconds) ; This node is disabled and will not be called.\nDrag off pins to build functionality.
)

(fn ConstructionScript
  (|CallParentFunction))