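; Base multiplayer game mode that tracks connected players and provides player spawning.
; Login and logout update the AllPlayers list and notify the game state; login also refreshes PlayersAlive from that list.
; SpawnPlayer destroys any controlled pawn, spawns a third-person character at a random PlayerStart and possesses it.
; NextLevel, StartLevel and controller swapping are empty, with random map-loading logic left disconnected.
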(event Custom|Update%20Player%20Alive
  ;[1 0 0] Update Alive player
  (Variables|Default|SetPlayers%20Alive (Variables|Default|GetAll%20Players)))

(event EventNextLevel
  ;[1 0 0] Next Level
)

(event EventPostLogin
  (params (NewPlayer :type Player%20Controller%20Object%20Reference))
  ;[0.03646 0.03646 0.03646] Player Connection / Disconnection
  ;;[1 1 1] Event connect player
  (Utilities|Array|Add (Variables|Default|GetAll%20Players) 0)
  (Class|BPIGameState|NotifyPlayerConnection(Message) (Game|GetGameState))
  (CallFunction|UpdatePlayerAlive))

(event EventOnSwapPlayerControllers
  (params (OldPC :type Player%20Controller%20Object%20Reference) (NewPC :type Player%20Controller%20Object%20Reference)))

(event EventOnLogout
  (params (ExitingController :type Controller%20Object%20Reference))
  ;[0.03646 0.03646 0.03646] Player Connection / Disconnection
  ;;[1 1 1] Event disconnect player
  (bind _asbp_pc_base_player_controller (Utilities|Casting|CastToBP_PC_BasePlayerController ExitingController))
  (Utilities|Array|RemoveItem (Variables|Default|GetAll%20Players) _asbp_pc_base_player_controller)
  (Class|BPIGameState|NotifyPlayerConnection(Message) (Game|GetGameState)))

(fn ConstructionScript)

(fn FindRandomPlayerStart
  (bind _outactors (Actor|GetAllActorsOfClass "/Script/Engine.PlayerStart"))
  (return (Transformation|GetActorTransform (Utilities|Array|Get(acopy) _outactors (Math|Random|RandomIntegerinRange 0 (- (Utilities|Array|Length _outactors) 1))))))

(fn SpawnPlayer
  (params (PlayerController :type Player%20Controller%20Object%20Reference))
  (bind _returnvalue (Pawn|GetControlledPawn PlayerController))
  (Utilities|IsValid _returnvalue
    (:Is%20Valid
      (Actor|DestroyActor _returnvalue))
    (:Is%20Not%20Valid
      _))
  (bind _returnvalue_2 (Game|SpawnActorfromClass "/Game/ThirdPerson/Blueprints/BP_ThirdPersonCharacter.BP_ThirdPersonCharacter_C" (Spawning|FindRandomPlayerStart) "Undefined" "MultiplyWithRoot" 0 0))
  (Pawn|Possess PlayerController _returnvalue_2))

(fn StartLevel)