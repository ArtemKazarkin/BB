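; Multiplayer base game state that tracks how many players remain and declares the last one standing the round winner.
; Connection and death notifications update the count; after a death, the authority takes the winner's name from the first remaining character and calls NextLevelMessage on the game mode.
; The WinnerName RepNotify shows the round result widget to the local player.
; Random map-loading logic is present but disconnected.
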(event Custom|CheckIfGameFinished?
  ;[1 1 1] CheckIfGameFinished
  (Networking|SwitchHasAuthority
    (:Authority
      (Utilities|FlowControl|Delay 0.2)
      (bind _outactors (Actor|GetAllActorsOfClass "/Game/ThirdPerson/Blueprints/BP_ThirdPersonCharacter.BP_ThirdPersonCharacter_C"))
      (if (== (Variables|Default|GetCurrent%20Amount%20of%20Players) 1)
        (Variables|Default|SetWinnerName (PlayerState|GetPlayerName (Variables|/Script/Engine.Pawn|GetPlayerState (Utilities|Array|Get(acopy) _outactors))))
        (Utilities|FlowControl|Delay 2.0)
        (Class|BPIGameMode|NextLevel(Message) (Game|GetGameMode))))))

(event EventNotifyPlayerDeath
  ;[1 1 1] Update alive player(Обновляем список живых игроков)
  (Variables|Default|SetCurrent%20Amount%20of%20Players (- (Variables|Default|GetCurrent%20Amount%20of%20Players) 1))
  (CallFunction|CheckifGameFinished?))

(event EventNotifyPlayerConnection
  (Variables|Default|SetCurrent%20Amount%20of%20Players (Class|GameplayStatics|GetNumPlayerStates)))

(fn ConstructionScript)

(fn OnRepWinnerName
  (if (not (Utilities|Array|IsEmpty (Variables|Default|GetWinnerName)))
    (if (Pawn|IsLocalPlayerController (Game|GetPlayerController 0))
      (bind _returnvalue (UserInterface|CreateWidget "/Game/UI/Game/WB_RoundResult.WB_RoundResult_C" (Game|GetPlayerController 0) (Variables|Default|GetWinnerName)))
      (UserInterface|Viewport|AddtoViewport _returnvalue 0))))