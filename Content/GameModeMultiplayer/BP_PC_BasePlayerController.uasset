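; Base multiplayer player controller that requests a pawn spawn for its player.
; On BeginPlay, the local controller calls the server spawn event and adds the default Enhanced Input mapping context.
; The server event casts the game mode to BP_GM_BaseGameMode and passes itself to SpawnPlayer.
; RespawnAllPlayer reuses the same spawn event for this controller.
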(event Custom|SR_SpawnPlayer
  ;[0 0 0] Spawn Player
  ;;[1 1 1] Server
  (bind _asbp_gm_base_game_mode (Utilities|Casting|CastToBP_GM_BaseGameMode (Game|GetGameMode)))
  (Default|SpawnPlayer _asbp_gm_base_game_mode self))

(event EventRespawnAllPlayer
  ;[1 1 1] RespawnAllPlayer
  (CallFunction|SRSpawnPlayer))

(event EventBeginPlay
  ;[0 0 0] Spawn Player
  ;;[1 1 1] Local
  (if (Pawn|IsLocalPlayerController)
    (CallFunction|SRSpawnPlayer)
    (Input|AddMappingContext (PlayerController|LocalPlayerSubsystems|GetEnhancedInputLocalPlayerSubsystem (Game|GetPlayerController 0)) "/Game/ThirdPerson/Input/IMC_Default.IMC_Default" 0 "(bIgnoreAllPressedKeysUntilRelease=True,bForceImmediately=False,bNotifyUserSettings=False)")))

(fn ConstructionScript)