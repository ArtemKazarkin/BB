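; BP_MissingPlatform is a world platform that vanishes shortly after something overlaps its trigger box, then returns.
; On overlap, the Cube's dynamic M_Bright material lights up while a Timeline animates its Opacity.
; After a delay the Cube is hidden and loses collision; after a second delay both are restored.
; A fresh material instance is created on return, resetting the look, and any overlapping actor triggers the cycle.
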(event OnComponentBeginOverlap(Box)
  (params (OverlappedComponent :type Primitive%20Component%20Object%20Reference) (OtherActor :type Actor%20Object%20Reference) (OtherComp :type Primitive%20Component%20Object%20Reference) (OtherBodyIndex :type Integer) (bFromSweep :type Boolean) (SweepResult :type Hit%20Result%20Structure%20%28by%20ref%29))
  (bind _cube (Variables|Default|GetCube))
  (bind _cube_2 (Variables|Default|GetCube))
  (Rendering|Material|SetScalarParameterValue (Variables|Default|GetDynamic%20Material) "Bright" 2.0 :!class /Script/Engine.MaterialInstanceDynamic)
  (Utilities|FlowControl|Sequence
    (:then_0
      (bind _newtrack_0 (Timeline|Timeline PlayFromStart)
        (:Update
          (Rendering|Material|SetScalarParameterValue (Variables|Default|GetDynamic%20Material) "Opacity" _newtrack_0 :!class /Script/Engine.MaterialInstanceDynamic))))
    (:then_1
      ;[1 1 1] Platform Visability Off
      (Utilities|FlowControl|Delay 3.0)
      (Rendering|SetVisibility _cube_2 false false)
      (Collision|SetCollisionEnabled _cube_2 "NoCollision")
      ;[1 1 1] Platform Visability On
      (Utilities|FlowControl|Delay 5.0)
      (bind _returnvalue (Rendering|Material|CreateDynamicMaterialInstance (Variables|Default|GetCube) 0 "/Game/WorldItems/Platforms/M_Bright.M_Bright" "None" :!class /Script/Engine.PrimitiveComponent))
      (bind _output_get (Variables|Default|SetDynamic%20Material _returnvalue))
      (Rendering|Material|SetScalarParameterValue _output_get "Bright" 0.0 :!class /Script/Engine.MaterialInstanceDynamic)
      (Rendering|SetVisibility _cube true false)
      (Collision|SetCollisionEnabled _cube "QueryAndPhysics"))))

(event EventBeginPlay
  (bind _returnvalue (Rendering|Material|CreateDynamicMaterialInstance (Variables|Default|GetCube) 0 "/Game/WorldItems/Platforms/M_Bright.M_Bright" "None" :!class /Script/Engine.PrimitiveComponent))
  (bind _output_get (Variables|Default|SetDynamic%20Material _returnvalue))
  (Rendering|Material|SetScalarParameterValue _output_get "Bright" 0.0 :!class /Script/Engine.MaterialInstanceDynamic))

(fn ConstructionScript)