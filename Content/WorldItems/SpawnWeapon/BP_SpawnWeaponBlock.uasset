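; BP_SpawnWeaponBlock is a world item that spawns a random weapon when its trigger box is overlapped.
; The box's begin overlap runs through a DoOnce that is never reset, so only the first overlap, by any actor, triggers a spawn.
; SpawnWeapon picks a random class from WeaponArray and spawns it at the world transform of the TransformWeapon component.
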(event OnComponentBeginOverlap(Box)
  (params (OverlappedComponent :type Primitive%20Component%20Object%20Reference) (OtherActor :type Actor%20Object%20Reference) (OtherComp :type Primitive%20Component%20Object%20Reference) (OtherBodyIndex :type Integer) (bFromSweep :type Boolean) (SweepResult :type Hit%20Result%20Structure%20%28by%20ref%29))
  (Utilities|FlowControl|DoOnce false
    (:Completed
      (CallFunction|SpawnWeapon))))

(fn ConstructionScript)

(fn SpawnWeapon
  (bind _output_get (Variables|Default|SetWeaponArray (Variables|Default|GetWeaponArray)))
  (Game|SpawnActorfromClass (Utilities|Array|Get(acopy) _output_get (Math|Random|RandomInteger (Utilities|Array|Length (Variables|Default|GetWeaponArray)))) (Transformation|GetWorldTransform (Variables|Default|GetTransformWeapon)) "Undefined" "MultiplyWithRoot" 0 0))